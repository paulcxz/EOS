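; Blueprint function library with pure math helpers for a character property set covering damage, armor, attributes, survival stats and their regen rates.
; LibPureSumProperties adds two property sets field by field.
; LibPureSubProperties subtracts P2 from P1 for damage, armor, attributes and current and max survival stats, but outputs zero for all four regen fields, so it is not a full inverse of the sum.
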(fn `LibPure_SubProperties`
  (params (P1 :type "/Game/Defend/Blueprints/Structures/S_Properties Structure") (P2 :type "/Game/Defend/Blueprints/Structures/S_Properties Structure"))
  (returns (P1MinusP2 :type "/Game/Defend/Blueprints/Structures/S_Properties Structure"))
  (bind (_damage_range _damage_melee _armor _strength _agility _intelligence _health _maxhealth _stamina _maxstamina _hunger _maxhunger _thirst _maxthirst) (break `/Game/Defend/Blueprints/Structures/S_Properties` P1))
  (bind (_damage_range_2 _damage_melee_2 _armor_2 _strength_2 _agility_2 _intelligence_2 _health_2 _maxhealth_2 _stamina_2 _maxstamina_2 _hunger_2 _maxhunger_2 _thirst_2 _maxthirst_2) (break `/Game/Defend/Blueprints/Structures/S_Properties` P2))
  (return (make `/Game/Defend/Blueprints/Structures/S_Properties` (- _damage_range _damage_range_2) (- _damage_melee _damage_melee_2) (- _armor _armor_2) (- _strength _strength_2) (- _agility _agility_2) (- _intelligence _intelligence_2) (- _health _health_2) (- _maxhealth _maxhealth_2) (- _stamina _stamina_2) (- _maxstamina _maxstamina_2) (- _hunger _hunger_2) (- _maxhunger _maxhunger_2) (- _thirst _thirst_2) (- _maxthirst _maxthirst_2))))

(fn `LibPure_SumProperties`
  (params (P1 :type "/Game/Defend/Blueprints/Structures/S_Properties Structure") (P2 :type "/Game/Defend/Blueprints/Structures/S_Properties Structure"))
  (returns (Result :type "/Game/Defend/Blueprints/Structures/S_Properties Structure"))
  (bind (_damage_range _damage_melee _armor _strength _agility _intelligence _health _maxhealth _stamina _maxstamina _hunger _maxhunger _thirst _maxthirst _regenhealth _regenstamina _regenhunger _regenthirst) (break `/Game/Defend/Blueprints/Structures/S_Properties` P1))
  (bind (_damage_range_2 _damage_melee_2 _armor_2 _strength_2 _agility_2 _intelligence_2 _health_2 _maxhealth_2 _stamina_2 _maxstamina_2 _hunger_2 _maxhunger_2 _thirst_2 _maxthirst_2 _regenhealth_2 _regenstamina_2 _regenhunger_2 _regenthirst_2) (break `/Game/Defend/Blueprints/Structures/S_Properties` P2))
  (return (make `/Game/Defend/Blueprints/Structures/S_Properties` (+ _damage_range_2 _damage_range) (+ _damage_melee_2 _damage_melee) (+ _armor_2 _armor) (+ _strength_2 _strength) (+ _agility_2 _agility) (+ _intelligence_2 _intelligence) (+ _health_2 _health) (+ _maxhealth_2 _maxhealth) (+ _stamina_2 _stamina) (+ _maxstamina_2 _maxstamina) (+ _hunger_2 _hunger) (+ _maxhunger _maxhunger_2) (+ _thirst_2 _thirst) (+ _maxthirst_2 _maxthirst) (+ _regenhealth _regenhealth_2) (+ _regenstamina_2 _regenstamina) (+ _regenhunger _regenhunger_2) (+ _regenthirst _regenthirst_2))))