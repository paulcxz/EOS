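; GM is the game mode blueprint for Defend, handling player respawning.
; On restart, it destroys the player's current pawn, then spawns a Pawn_L4_PlayerPawn at a random PlayerStart and possesses it.
; The random index uses length minus one as an exclusive maximum, so with multiple starts the last one is never picked.
; BeginPlay and Tick are empty, and a CreatePlayer call is left unconnected.
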(event `self.ReceiveBeginPlay`)

(event `self.K2_OnRestartPlayer`
  (params (NewPlayer :type "Controller Object Reference"))
  (bind _returnvalue (`Controller.K2_GetPawn` NewPlayer))
  (`/Engine/EditorBlueprintResources/StandardMacros.IsValid` _returnvalue
    (:`Is Valid`
      (`self.K2_DestroyActor` _returnvalue))
    (:`Is Not Valid`
      _))
  (bind _outactors (`GameplayStatics.GetAllActorsOfClass` "/Script/Engine.PlayerStart"))
  (bind _returnvalue_2 (`|SpawnActorFromClass` "/Game/Defend/Blueprints/Pawns/Pawn_L4_PlayerPawn.Pawn_L4_PlayerPawn_C" (`self.GetTransform` (`|GetArrayItem` _outactors (`KismetMathLibrary.RandomInteger` (- (`KismetArrayLibrary.Array_Length` _outactors) 1)))) "AdjustIfPossibleButAlwaysSpawn" "OverrideRootScale" null null))
  (`Controller.Possess` NewPlayer _returnvalue_2))

(fn `UserConstructionScript`)