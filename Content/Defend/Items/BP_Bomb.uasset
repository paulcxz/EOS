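; BP_Bomb is an explosive actor that detonates almost immediately after spawning and then destroys itself.
; After a brief delay on BeginPlay, it sends a damage interface message to every actor overlapping its Sphere, with damage falling off linearly by distance from the bomb.
; It prints each damage value as debug text, then fires a RadialForce impulse for the physical blast.
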(event `self.ReceiveBeginPlay`
  (`KismetSystemLibrary.Delay` 0.05)
  (for _array_element (`PrimitiveComponent.GetOverlappingActors` (`self.Sphere`) null)
    (bind _returnvalue (`KismetMathLibrary.MapRangeClamped` (`KismetMathLibrary.Vector_Distance` (`self.K2_GetActorLocation` _array_element) (`self.K2_GetActorLocation`)) 0.0 500.0 500.0 75.0))
    (`KismetSystemLibrary.PrintString` (`KismetStringLibrary.Conv_DoubleToString` _returnvalue) true true (struct :`R` 1.0 :`G` 0.074398 :`A` 1.0) 1111.0)
    (message `/Game/Defend/Blueprints/Interfaces/I_Damageable.I_TakeDamage` _array_element _returnvalue "NewEnumerator3" self (`self.K2_GetActorLocation`)))
  (`RadialForceComponent.FireImpulse` (`self.RadialForce`))
  (`self.K2_DestroyActor`))

(fn `UserConstructionScript`)