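; BP_EffectBase is the base actor for timed consumable item effects applied to a Pawn.
; On BeginPlay it registers with the Pawn if PureCanItemBeUsed passes, otherwise it destroys itself; the base check returns false.
; Tick drives FuncEffectProgress with normalized elapsed time over Duration, then destroys the actor at completion.
; The progress function is empty, leaving both it and the usability check as hooks for child effects.
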(event `self.ReceiveBeginPlay`
  (if (`self.Pure_CanItemBeUsed`)
    (`/Game/Defend/Blueprints/Pawns/Pawn_L2_AdvLocom.Func_AddEffect` (`self.Pawn`) self)
    (`self.Func_EffectProgress` 0.0)
    (else
      (`self.K2_DestroyActor`))))

(event `self.ReceiveTick`
  (params (DeltaSeconds :type "Float (single-precision)"))
  (bind _output_get (set `self.TimeElapsed` (`KismetMathLibrary.FClamp` (+ (stale _output_get) DeltaSeconds) 0.0 (`self.Duration`))))
  (if (< (`self.TimeElapsed`) (`self.Duration`))
    (`self.Func_EffectProgress` (/ (`self.TimeElapsed`) (`self.Duration`)))
    (else
      (`self.Func_EffectProgress` 1.0)
      (`self.K2_DestroyActor`))))

(fn `Func_EffectProgress`
  (params (Progress :type "Float (double-precision)")))

(fn `Pure_CanItemBeUsed`
  (returns (ReturnValue :type Boolean))
  (return false))

(fn `UserConstructionScript`)