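; M4A1 equippable weapon that fires automatically while the trigger is held and the owner is aiming.
; Each shot spends ammo, shows particles, relays "Shoot" to the owner, then re-fires after a cooldown.
; A screen-center trace draws a debug sphere, then damages and spawns BP_Bomb on hits, sparing team 0.
; Reload requests go to the owner, but inventory counting and refill logic are disconnected.
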(event `self.ReceiveBeginPlay`
  (`parent.ReceiveBeginPlay`)
  (bind _returnvalue (`|GetDataTableRow` "/Game/Defend/Datatables/ItemList.ItemList" (`self.AmmoID`))
    (:`then`
      (set `self.Properties` (`.Properties_129_A634906B4553FCCD99B0D8ABE8DBB8D9` (break `/Game/Defend/Blueprints/Structures/InventoryItem` _returnvalue))))))

(event `/Game/Defend/Blueprints/Interfaces/I_HandEquipmentRelative.I_SecondAction`
  (params (Pressed :type Boolean))
  (bind _output_get (set `self.Aiming` Pressed))
  (message `/Game/Defend/Blueprints/Interfaces/I_HandEquipmentRelative.I_RecallAction` (`self.ItemOwner`) "Aim" _output_get))

(event `/Game/Defend/Blueprints/Interfaces/I_HandEquipmentRelative.I_RecallAction`
  (params (ActionName :type Name) (ActionBegin :type Boolean))
  (`self.Func_OnRecall` ActionName ActionBegin))

(event `/Game/Defend/Blueprints/Interfaces/I_HandEquipmentRelative.I_MainAction`
  (params (Pressed :type Boolean))
  (bind _output_get (set `self.TriggerPressed` Pressed))
  (if _output_get
    (`self.CE_OneShot`)))

(event `/Game/Defend/Blueprints/Interfaces/I_HandEquipmentRelative.I_ThirdAction`
  (params (Pressed :type Boolean))
  (bind (_ammoininventory _ammoneeded) (`self.Pure_GetReloadInfo`))
  (if Pressed
    (if (and (> _ammoininventory 0) (> _ammoneeded 0))
      (message `/Game/Defend/Blueprints/Interfaces/I_HandEquipmentRelative.I_RecallAction` (`self.ItemOwner`) "Reload" true))))

(event `CE_OneShot`
  (if (`self.Pure_CanShot`)
    (bind _succ (`self.Func_FireTheBullet`))
    (if _succ
      (`self.Func_ApplyDamageOnTarget`)
      (`KismetSystemLibrary.Delay` (`self.CD`))
      (`self.Func_OnCooldown`)
      (else
        (`GameplayStatics.SpawnSoundAttached` "/Game/Sounds/NoAmmo.NoAmmo" (`self.Muzzle`) "None" (0.0 0.0 0.0) (struct) "KeepRelativeOffset" false 1.0 1.0 0.0 null null)
        (`SceneComponent.SetVisibility` (`self.ParticleSystem`) false false :!label _label)))
    (else
      (goto _label))))

(fn `Func_ApplyDamageOnTarget`
  (returns (TargetExists :type Boolean))
  (locals (l_HitActor :type "Actor Object Reference") (l_VoxelWorld :type "Object Object Reference") (l_HitLocation :type "Vector Structure" :default (0.0 0.0 0.0)))
  (bind _asplayer_controller (`self.Pure_GetOwnerPC`))
  (bind _itemowner (`self.ItemOwner`))
  (bind (_hitresult _returnvalue) (`CXZFuncLib.CXZLineTraceFromScreenPosPercentage` :`Player` _asplayer_controller :`TraceChannel` "TraceTypeQuery1" :`bTraceComplex` true :`x` 0.5 :`y` 0.5))
  (bind (_bblockinghit _binitialoverlap _time _distance _location _impactpoint _normal _impactnormal _physmat _hitactor) (`GameplayStatics.BreakHitResult` _hitresult))
  (`/Engine/EditorBlueprintResources/StandardMacros.IsValid` _asplayer_controller
    (:`Is Valid`
      (if _returnvalue
        (bind _output_get (set `local.l_HitLocation` _location))
        (`KismetSystemLibrary.DrawDebugSphere` _output_get 10.0 12 (struct :`R` 1.0 :`A` 1.0) 3.0 1.0)
        (bind _output_get_2 (set `local.l_HitActor` _hitactor))
        (if (`KismetSystemLibrary.DoesImplementInterface` _output_get_2 "/Game/Defend/Blueprints/Interfaces/I_Team.I_Team_C")
          (bind _id (message `/Game/Defend/Blueprints/Interfaces/I_Team.I_GetTeamID` (`local.l_HitActor`)))
          (if (!= _id 0)
            _
            (else
              (return true))))
        (message `/Game/Defend/Blueprints/Interfaces/I_Damageable.I_TakeDamage` (`local.l_HitActor`) (`.Damage_Range_2_8221955E4E575A8C65DD158F464D07F7` (break `/Game/Defend/Blueprints/Structures/S_Properties` (`/Game/Defend/Blueprints/Pawns/Pawn_L2_AdvLocom.Pure_GetProperties` (cast `/Game/Defend/Blueprints/Pawns/Pawn_L2_AdvLocom` (`self.ItemOwner`) :!pure true)))) "NewEnumerator1" _itemowner (0.0 0.0 0.0))
        (`|SpawnActorFromClass` "/Game/Defend/Items/BP_Bomb.BP_Bomb_C" (`KismetMathLibrary.MakeTransform` (`local.l_HitLocation`)) "AlwaysSpawn" "OverrideRootScale" null (cast `Pawn` _itemowner :!pure true))
        (return true)
        (else
          _)))
    (:`Is Not Valid`
      _))
  (return false))

(fn `Func_BeenInteracted`
  (params (ByWhom :type "Actor Object Reference")))

(fn `Func_FireTheBullet`
  (returns (Succ :type Boolean))
  (if (> (`self.Ammo`) 0)
    (`ActorComponent.SetActive` (`self.ParticleSystem`) true false)
    (`SceneComponent.SetVisibility` (`self.ParticleSystem`) true false)
    (`/Engine/EditorBlueprintResources/StandardMacros.DecrementInt` (`self.Ammo`)
      (:`  `
        (set `self.Cooldown` false)
        (message `/Game/Defend/Blueprints/Interfaces/I_HandEquipmentRelative.I_RecallAction` (`self.ItemOwner`) "Shoot" true)
        (return true)))
    (else
      (return false))))

(fn `Func_OnCooldown`
  (set `self.Cooldown` true)
  (`SceneComponent.SetVisibility` (`self.ParticleSystem`) false false)
  (if (`self.TriggerPressed`)
    (`self.CE_OneShot`)))

(fn `Func_OnRecall`
  (params (ActionName :type Name) (ActionBegin :type Boolean))
  (locals (l_AmmoCost :type Integer)))

(fn `Func_Pickup`
  (params (ByWhom :type "Actor Object Reference"))
  (bind _staticmeshcomponent (`self.StaticMeshComponent`))
  (`PrimitiveComponent.SetSimulatePhysics` _staticmeshcomponent false)
  (`PrimitiveComponent.SetCollisionEnabled` _staticmeshcomponent "NoCollision"))

(fn `I_GetAmmoID`
  (returns (ID :type Name))
  (return (`self.AmmoID`)))

(fn `I_GetAttachType`
  (returns (AttachType :type "/Game/Defend/Blueprints/Structures/E_AttachType Enum"))
  (return "NewEnumerator0"))

(fn `I_GetOverlayState`
  (returns (ReturnValue :type "/Game/AdvancedLocomotionV4/Data/Enums/ALS_OverlayState Enum"))
  (return "NewEnumerator1"))

(fn `Pure_CanShot`
  (returns (ReturnValue :type Boolean))
  (return (and (`self.Cooldown`) (`self.Aiming`) (`KismetSystemLibrary.IsValid` (`self.ItemOwner`)))))

(fn `Pure_GetAmmoInInventory`
  (params (ID :type Name))
  (returns (Ammo :type Integer))
  (locals (l_AmmoIHave :type Integer)))

(fn `Pure_GetReloadInfo`
  (returns (AmmoInInventory :type Integer) (AmmoNeeded :type Integer))
  (locals (l_AmmoNeeded :type Integer) (l_AmmoIHave :type Integer))
  (`|ExecutionSequence`
    (:`then_0`
      (bind _output_get (set `local.l_AmmoNeeded` (- (`self.MaxAmmo`) (`self.Ammo`))))
      (if (> _output_get 0)
        (set `local.l_AmmoIHave` (`self.Pure_GetAmmoInInventory` (`self.AmmoID`)))))
    (:`then_1`
      (return (`local.l_AmmoIHave`) (`local.l_AmmoNeeded`)))))

(fn `UserConstructionScript`
  (`parent.UserConstructionScript`))