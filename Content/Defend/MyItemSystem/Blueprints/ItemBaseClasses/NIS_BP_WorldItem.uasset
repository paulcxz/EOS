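; Base world item actor that represents an item from the item data table and destroys itself when picked up.
; The construction script looks up ItemID, fills ItemInfo with a new GUID and definition, and optionally randomizes quality, stack amount and a bounce value.
; It then sets the static mesh and fits the box to its bounds with a minimum size.
; Interface and helper functions expose ItemInfo and the owner's PlayerController.
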(event `/Game/Defend/MyItemSystem/Blueprints/Interfaces/NIS_I_WorldItem.I_PickedUp`
  (params (Who :type "Pawn Object Reference"))
  (`self.K2_DestroyActor`))

(fn `Func_RandomizeItem`
  (bind ((`MinQuality_140_6772D6FA4A2CDC455A1F62B5307EA515` _minquality) (`MaxQuality_135_CBD1FAA54940E088B192D7A42622FDA0` _maxquality) (`MaxStackSize_105_457804EE421C991C4D20ADA6928E4B40` _maxstacksize)) (break `/Game/Defend/MyItemSystem/Structs/NIS_S_ItemDefination` (`.Definiation_2_5F261EEE43996261C586B7A249020746` (break `/Game/Defend/MyItemSystem/Structs/NIS_S_Item` (`self.ItemInfo`)))))
  (if (`self.Randomize`)
    (setmembers `/Game/Defend/MyItemSystem/Structs/NIS_S_Item` :`StructRef` (`self.ItemInfo`) :`CurrentState` (make `/Game/Defend/MyItemSystem/Structs/NIS_S_ItemCurrentState` (cast `/Game/Defend/MyItemSystem/Structs/NIC_E_ItemQuality` (`KismetMathLibrary.Conv_IntToByte` (`KismetMathLibrary.RandomIntegerInRange` (`KismetMathLibrary.Conv_ByteToInt` _minquality) (`KismetMathLibrary.Conv_ByteToInt` _maxquality)))) (`KismetMathLibrary.RandomIntegerInRange` 1 _maxstacksize) (`KismetMathLibrary.RandomFloatInRange` 0.5 1.5)))))

(fn `I_GetItemInfo`
  (returns (ItemInfo :type "/Game/Defend/MyItemSystem/Structs/NIS_S_Item Structure"))
  (return (`self.ItemInfo`)))

(fn `Pure_GetOwnerPC`
  (returns (`AsPlayer Controller` :type "PlayerController Object Reference"))
  (bind _aspawn (cast `Pawn` (`self.ItemOwner`))
    (:`then`
      (bind _asplayer_controller (cast `PlayerController` (`Pawn.GetController` _aspawn))
        (:`then`
          (return _asplayer_controller))
        (:`CastFailed`
          _)))
    (:`CastFailed`
      _))
  (return null))

(fn `UserConstructionScript`
  (locals (l_MinTriggerBoxEdgeLength :type "Float (double-precision)" :default 20.0))
  (bind _l_mintriggerboxedgelength (`local.l_MinTriggerBoxEdgeLength`))
  (bind _box (`self.Box`))
  (bind (_origin _boxextent) (`KismetSystemLibrary.GetComponentBounds` (`self.StaticMeshComponent`)))
  (bind _returnvalue (`|GetDataTableRow` "/Game/Defend/MyItemSystem/Data/NIS_DT_Itemlist.NIS_DT_Itemlist" (`self.ItemID`))
    (:`then`
      (setmembers `/Game/Defend/MyItemSystem/Structs/NIS_S_Item` :`StructRef` (`self.ItemInfo`) :`Valid` true :`ItemGUID` (`KismetGuidLibrary.NewGuid`) :`Definiation` _returnvalue)
      (`self.Func_RandomizeItem`)
      (`StaticMeshComponent.SetStaticMesh` (`self.StaticMeshComponent`) (`.WorldStaticMesh_147_4B150C904AFC21226059E49567A144DC` (break `/Game/Defend/MyItemSystem/Structs/NIS_S_ItemDefination` (`.Definiation_2_5F261EEE43996261C586B7A249020746` (break `/Game/Defend/MyItemSystem/Structs/NIS_S_Item` (`self.ItemInfo`))))))
      (`SceneComponent.K2_SetWorldLocation` _box _origin false false)
      (`BoxComponent.SetBoxExtent` _box (`KismetMathLibrary.MakeVector` (`KismetMathLibrary.FMax` (.x _boxextent) _l_mintriggerboxedgelength) (`KismetMathLibrary.FMax` (.y _boxextent) _l_mintriggerboxedgelength) (`KismetMathLibrary.FMax` (.z _boxextent) _l_mintriggerboxedgelength)) true))))