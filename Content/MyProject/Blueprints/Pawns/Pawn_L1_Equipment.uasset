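; Pawn layer that handles replicated equipment visuals, equipment stat totals and inventory actions through NIS.
; RepNotify meshes make worn pieces follow the body via master pose, while rings, hand items and trinket snap to sockets.
; Capsule overlap auto-picks up consumables, currency and ammo, offering them to inventories in order until one accepts; ROS events also handle move and drop.
; Equipment totals sum each item's base properties adjusted by its randomized bounce.
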(event `self.ReceiveBeginPlay`)

(event `self.CapsuleComponent.OnComponentBeginOverlap`
  (params (OverlappedComponent :type "PrimitiveComponent Object Reference") (OtherActor :type "Actor Object Reference") (OtherComp :type "PrimitiveComponent Object Reference") (OtherBodyIndex :type Integer) (bFromSweep :type Boolean) (SweepResult :type "HitResult Structure (by ref)"))
  ;[1 1 1] 如果碰到一个可以自动拾取的物品则自动拾取它
  (bind _asnis_bp_world_item (cast `/Game/MyProject/MyItemSystem/Blueprints/ItemBaseClasses/NIS_BP_WorldItem` OtherActor))
  (bind _iteminfo (message `/Game/MyProject/MyItemSystem/Blueprints/Interfaces/NIS_I_WorldItem.I_GetItemInfo` _asnis_bp_world_item))
  (switch `/Game/MyProject/MyItemSystem/Structs/NIS_E_ItemType` (`.ItemType_136_6F65BDF74AF3950358D25783E49E9C6F` (break `/Game/MyProject/MyItemSystem/Structs/NIS_S_ItemDefination` (`.Definiation_2_5F261EEE43996261C586B7A249020746` (break `/Game/MyProject/MyItemSystem/Structs/NIS_S_Item` _iteminfo))))
    (:`NewEnumerator0`
      _)
    (:`NewEnumerator7`
      _)
    (:`NewEnumerator8`
      _))
  (`self.ROS_PickUpItem` _asnis_bp_world_item))

(event `ROS_PickUpItem`
  (params (WorldItem :type "/Game/MyProject/MyItemSystem/Blueprints/ItemBaseClasses/NIS_BP_WorldItem Object Reference"))
  (`self.Server_PickUpItem` WorldItem))

(event `ROS_MoveItem`
  (params (FromInv :type "/Game/MyProject/MyItemSystem/Blueprints/NIS_Inventory Object Reference") (ToInv :type "/Game/MyProject/MyItemSystem/Blueprints/NIS_Inventory Object Reference") (FromSlot :type Integer) (ToSlot :type Integer) (Split :type Boolean))
  ;[1 1 1] NIS
  (`/Game/MyProject/MyItemSystem/Blueprints/Libraries/NIS_BFL.NIS_BFL_MoveItem` FromInv ToInv FromSlot ToSlot Split))

(event `ROS_DropItem`
  (params (FromInventory :type "/Game/MyProject/MyItemSystem/Blueprints/NIS_Inventory Object Reference") (Slot :type Integer))
  ;[1 1 1] NIS
  (`/Game/MyProject/MyItemSystem/Blueprints/Libraries/NIS_BFL.NIS_BFL_DropItem` FromInventory Slot))

(fn `Func_UpdateEquipProperties`
  (set `self.EquipmentsTotalProperties` (`self.Pure_GetTotalPropertiesFromEquipments`)))

(fn `OnRep_AccessoryMesh`
  (`SkinnedMeshComponent.SetSkinnedAssetAndUpdate` (`self.Accessory`) (`self.AccessoryMesh`) true)
  (`SkinnedMeshComponent.SetLeaderPoseComponent` (`self.Accessory`) (`self.Mesh`) false))

(fn `OnRep_BackMesh`
  (`SkinnedMeshComponent.SetSkinnedAssetAndUpdate` (`self.Back`) (`self.BackMesh`) true)
  (`SkinnedMeshComponent.SetLeaderPoseComponent` (`self.Back`) (`self.Mesh`) false))

(fn `OnRep_ChestMesh`
  (`SkinnedMeshComponent.SetSkinnedAssetAndUpdate` (`self.Chest`) (`self.ChestMesh`) true)
  (`SkinnedMeshComponent.SetLeaderPoseComponent` (`self.Chest`) (`self.Mesh`) false))

(fn `OnRep_FeetMesh`
  (`SkinnedMeshComponent.SetSkinnedAssetAndUpdate` (`self.Feet`) (`self.FeetMesh`) true)
  (`SkinnedMeshComponent.SetLeaderPoseComponent` (`self.Feet`) (`self.Mesh`) false))

(fn `OnRep_HandsMesh`
  (`SkinnedMeshComponent.SetSkinnedAssetAndUpdate` (`self.Hands`) (`self.HandsMesh`) true)
  (`SkinnedMeshComponent.SetLeaderPoseComponent` (`self.Hands`) (`self.Mesh`) false))

(fn `OnRep_HeadMesh`
  (`SkinnedMeshComponent.SetSkinnedAssetAndUpdate` (`self.Head`) (`self.HeadMesh`) true)
  (`SkinnedMeshComponent.SetLeaderPoseComponent` (`self.Head`) (`self.Mesh`) false))

(fn `OnRep_LeftRingMesh`
  (locals (LocalEquipmentSockets :type "/Game/MyProject/Blueprints/Structures/EquipmentSockets Structure" :default (struct :`RightRing` "RightRing" :`LeftRing` "LeftRing" :`Main-Hand` "MainHand" :`Off-Hand` "OffHand")))
  (`SkinnedMeshComponent.SetSkinnedAssetAndUpdate` (`self.LeftRing`) (`self.LeftRingMesh`) true)
  (`SceneComponent.K2_AttachToComponent` (`self.LeftRing`) (`self.Mesh`) (`.LeftRing_10_66512035469F61C34EC98F90E4F97407` (break `/Game/MyProject/Blueprints/Structures/EquipmentSockets` (`local.LocalEquipmentSockets`))) "SnapToTarget" "SnapToTarget" "SnapToTarget" true))

(fn `OnRep_LegsMesh`
  (`SkinnedMeshComponent.SetSkinnedAssetAndUpdate` (`self.Legs`) (`self.LegsMesh`) true)
  (`SkinnedMeshComponent.SetLeaderPoseComponent` (`self.Legs`) (`self.Mesh`) false))

(fn `OnRep_MainHandMesh`
  (locals (LocalEquipmentSockets :type "/Game/MyProject/Blueprints/Structures/EquipmentSockets Structure" :default (struct :`RightRing` "RightRing" :`LeftRing` "LeftRing" :`Main-Hand` "MainHand" :`Off-Hand` "OffHand")))
  (`SkinnedMeshComponent.SetSkinnedAssetAndUpdate` (`self.MainHand`) (`self.MainHandMesh`) true)
  (`SceneComponent.K2_AttachToComponent` (`self.MainHand`) (`self.Mesh`) (`.Main-Hand_14_8A558B7C43EA00D3972964BA4E935F53` (break `/Game/MyProject/Blueprints/Structures/EquipmentSockets` (`local.LocalEquipmentSockets`))) "SnapToTarget" "SnapToTarget" "SnapToTarget" true))

(fn `OnRep_OffHandMesh`
  (locals (LocalEquipmentSockets :type "/Game/MyProject/Blueprints/Structures/EquipmentSockets Structure" :default (struct :`RightRing` "RightRing" :`LeftRing` "LeftRing" :`Main-Hand` "MainHand" :`Off-Hand` "OffHand")))
  (`SkinnedMeshComponent.SetSkinnedAssetAndUpdate` (`self.OffHand`) (`self.OffHandMesh`) true)
  (`SceneComponent.K2_AttachToComponent` (`self.OffHand`) (`self.Mesh`) (`.Off-Hand_13_B721A1014D6248471814A7BBC96B4643` (break `/Game/MyProject/Blueprints/Structures/EquipmentSockets` (`local.LocalEquipmentSockets`))) "SnapToTarget" "SnapToTarget" "SnapToTarget" true))

(fn `OnRep_RightRingMesh`
  (locals (LocalEquipmentSockets :type "/Game/MyProject/Blueprints/Structures/EquipmentSockets Structure" :default (struct :`RightRing` "RightRing" :`LeftRing` "LeftRing" :`Main-Hand` "MainHand" :`Off-Hand` "OffHand")))
  (`SkinnedMeshComponent.SetSkinnedAssetAndUpdate` (`self.RightRing`) (`self.RightRingMesh`) true)
  (`SceneComponent.K2_AttachToComponent` (`self.RightRing`) (`self.Mesh`) (`.RightRing_5_1FCB62154ABF504F5383A3B8EA5B0E39` (break `/Game/MyProject/Blueprints/Structures/EquipmentSockets` (`local.LocalEquipmentSockets`))) "SnapToTarget" "SnapToTarget" "SnapToTarget" true))

(fn `OnRep_ShoulderMesh`
  (`SkinnedMeshComponent.SetSkinnedAssetAndUpdate` (`self.Shoulder`) (`self.ShoulderMesh`) true)
  (`SkinnedMeshComponent.SetLeaderPoseComponent` (`self.Shoulder`) (`self.Mesh`) false))

(fn `OnRep_TrinketMesh`
  (`SkinnedMeshComponent.SetSkinnedAssetAndUpdate` (`self.Trinket`) (`self.TrinketMesh`) true)
  (`SceneComponent.K2_AttachToComponent` (`self.Trinket`) (`self.Mesh`) "TrinketSock" "SnapToTarget" "SnapToTarget" "SnapToTarget" true))

(fn `OnRep_WaistMesh`
  (`SkinnedMeshComponent.SetSkinnedAssetAndUpdate` (`self.Waist`) (`self.WaistMesh`) true)
  (`SkinnedMeshComponent.SetLeaderPoseComponent` (`self.Waist`) (`self.Mesh`) false))

(fn `Pure_GetTotalPropertiesFromEquipments`
  (returns (Properties :type "/Game/MyProject/Blueprints/Structures/S_Properties Structure"))
  (locals (l_Sum :type "/Game/MyProject/Blueprints/Structures/S_Properties Structure"))
  (for _array_element (`self.EquipedItemsReference`)
    (`/Engine/EditorBlueprintResources/StandardMacros.IsValid` _array_element
      (:`Is Valid`
        (bind ((`Definiation_2_5F261EEE43996261C586B7A249020746` _definiation) (`CurrentState_12_E59680B04DB3FFA39D4B878CDD56837B` _currentstate)) (break `/Game/MyProject/MyItemSystem/Structs/NIS_S_Item` (`/Game/MyProject/MyItemSystem/Blueprints/ItemBaseClasses/NIS_BP_WorldItem.ItemInfo` _array_element)))
        (set `local.l_Sum` (`/Game/MyProject/Blueprints/BFL_CXZ.LibPure_SumProperties` (`/Game/MyProject/Blueprints/BFL_CXZ.LibPure_BounceProperty` (`.BasicProperties_141_A634906B4553FCCD99B0D8ABE8DBB8D9` (break `/Game/MyProject/MyItemSystem/Structs/NIS_S_ItemDefination` _definiation)) (`.RandomizedPropBounce_144_C7847BCA4F2E2B52E29F93ADCC5D1D6D` (break `/Game/MyProject/MyItemSystem/Structs/NIS_S_ItemCurrentState` _currentstate))) (`local.l_Sum`))))))
  (return (`local.l_Sum`)))

(fn `Server_PickUpItem`
  (params (Item :type "Object Object Reference"))
  (locals (l_ItemInfo :type "/Game/MyProject/MyItemSystem/Structs/NIS_S_Item Structure") (l_AddItemSucc :type Boolean :default false))
  (bind _iteminfo (message `/Game/MyProject/MyItemSystem/Blueprints/Interfaces/NIS_I_WorldItem.I_GetItemInfo` (`local.Item`)))
  (set `local.l_ItemInfo` _iteminfo)
  (for _array_element (`/Game/MyProject/MyItemSystem/Blueprints/Libraries/NIS_BFL.NIS_BFL_GetInventoriesInOrder` self)
    (bind _result (`/Game/MyProject/MyItemSystem/Blueprints/NIS_Inventory.Func_Server_AddItem` _array_element (`local.l_ItemInfo`) -1))
    (if _result
      (set `local.l_AddItemSucc` true)
      (break)))
  (if (`local.l_AddItemSucc`)
    (message `/Game/MyProject/MyItemSystem/Blueprints/Interfaces/NIS_I_WorldItem.I_PickedUp` (`local.Item`) self)))

(fn `UserConstructionScript`)