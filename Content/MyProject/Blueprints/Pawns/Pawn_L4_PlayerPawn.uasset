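; Player pawn that adds interaction, item pickup, equipment, team ID and death handling to its parent.
; Interact sends a debounced screen-center trace to the server, which uses an interactable in range or otherwise picks up overlapping world items.
; Equipment changes spawn the slot's item and equip weapons, or reset the overlay state when certain slots empty.
; Death drops every inventory item server-side and requests a delayed respawn from the controller.
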(event `self.ReceiveTick`
  (params (DeltaSeconds :type "Float (single-precision)"))
  (`parent.ReceiveTick` DeltaSeconds))

(event `Key|NumPadFive`
  (params (Key :type "Key Structure"))
  (:`Pressed`
    (`/Game/AdvancedLocomotionV4/Blueprints/Interfaces/ALS_Character_BPI.BPI_Set_ViewMode` "NewEnumerator1")))

(event `Server_PickupAllOverLappingItems`
  (bind _overlappingactors (`PrimitiveComponent.GetOverlappingActors` (`self.PickupCollision`) "/Game/MyProject/MyItemSystem/Blueprints/ItemBaseClasses/NIS_BP_WorldItem.NIS_BP_WorldItem_C"))
  (`/Engine/EditorBlueprintResources/ActorMacros.Switch Has Authority`
    (:`Authority`
      (`KismetSystemLibrary.PrintString` (`KismetStringLibrary.Conv_IntToString` (`KismetArrayLibrary.Array_Length` _overlappingactors)))
      (for _array_element _overlappingactors
        (bind _asnis_bp_world_item (cast `/Game/MyProject/MyItemSystem/Blueprints/ItemBaseClasses/NIS_BP_WorldItem` _array_element))
        (`self.ROS_PickUpItem` _asnis_bp_world_item)))
    (:`Remote`
      (`KismetSystemLibrary.PrintString` "123123"))))

(event `InputAction|Interact`
  (params (Key :type "Key Structure"))
  (:`Pressed`
    (`/Engine/EditorBlueprintResources/StandardMacros.Gate` false :!label _label
      (:`Exit`
        (`|ExecutionSequence`
          (:`then_0`
            (`self.ROS_Interact` (`CXZFuncLib.CXZLineTraceFromScreenPosPercentage` (cast `PlayerController` (`self.GetController`) :!pure true) "TraceTypeQuery1" (`|MakeArray` self :!type "Actor Object Reference") true true 0.5 0.5)))
          (:`then_1`
            (goto _label :!via `Close`))
          (:`then_2`
            (`KismetSystemLibrary.Delay` 0.02)
            (goto _label :!via `Open`)))))))

(event `ROS_Interact`
  (params (Hit :type "HitResult Structure"))
  (`self.FuncServer_Interact` Hit))

(event `Key|T`
  (params (Key :type "Key Structure"))
  (:`Pressed`
    (bind _outactors (`GameplayStatics.GetAllActorsOfClass` "/Game/MyProject/Items/EquipableItemActors/BP_Weapon_M4A1.BP_Weapon_M4A1_C"))
    (message `/Game/MyProject/Blueprints/Interfaces/UsableActorInterface.OnActorUsed` (`|GetArrayItem` _outactors) self)))

(event `/Game/MyProject/Blueprints/Interfaces/I_EquippedPawn.I_EquipmentChanged`
  (params (ChangedSlot :type "/Game/MyProject/Blueprints/Structures/NIS_E_EquipmentSlotID Enum" :default "NewEnumerator0"))
  (`self.Func_EquipmentChanged` ChangedSlot))

(event `/Game/MyProject/Blueprints/Interfaces/I_Team.I_SetTeamID`
  (params (ID :type Integer))
  (bind _output_get (set `self.TeamID` ID))
  (`KismetSystemLibrary.PrintString` (`KismetStringLibrary.Conv_IntToString` _output_get) true true (struct :`R` 1.0 :`G` 0.874468 :`A` 1.0) 122.0))

(fn `Func_EquipmentChanged`
  (params (Slot :type "/Game/MyProject/Blueprints/Structures/NIS_E_EquipmentSlotID Enum" :default "NewEnumerator0"))
  (locals (l_NewItemInfo :type "/Game/MyProject/MyItemSystem/Structs/NIS_S_Item Structure") (l_NewSpawnItem :type "/Game/MyProject/MyItemSystem/Blueprints/ItemBaseClasses/NIS_BP_WorldItem Object Reference"))
  (bind _slot (`local.Slot`))
  (bind ((`ID_35_21A6C172469948671FD3CB8A1BBED0DB` _id) (`ItemSubClass_143_C5B5C66D47329B73D4F63CB32A844510` _itemsubclass)) (break `/Game/MyProject/MyItemSystem/Structs/NIS_S_ItemDefination` (`.Definiation_2_5F261EEE43996261C586B7A249020746` (break `/Game/MyProject/MyItemSystem/Structs/NIS_S_Item` (`|GetArrayItem` (`/Game/MyProject/MyItemSystem/Blueprints/NIS_Inventory.Pure_GetItems` (`self.Equipments`)) (`KismetMathLibrary.Conv_ByteToInt` (`local.Slot`)))))))
  (set `local.l_NewItemInfo` (`|GetArrayItem` (`/Game/MyProject/MyItemSystem/Blueprints/NIS_Inventory.Pure_GetItems` (`self.Equipments`)) (`KismetMathLibrary.Conv_ByteToInt` (`local.Slot`))))
  (if (`.Valid_10_A5F4438E4CED4CA4C4B5889683E540DA` (break `/Game/MyProject/MyItemSystem/Structs/NIS_S_Item` (`local.l_NewItemInfo`)))
    (`/Engine/EditorBlueprintResources/StandardMacros.IsValid` (`|GetArrayItem` (`self.EquipedItemsReference`) (`KismetMathLibrary.Conv_ByteToInt` (`local.Slot`)))
      (:`Is Not Valid`
        (bind _returnvalue (`|SpawnActorFromClass` _itemsubclass (`KismetMathLibrary.MakeTransform` (0.0 0.0 0.0)) "Undefined" "OverrideRootScale" null _id false null))
        (bind _output_get (set `local.l_NewSpawnItem` _returnvalue))
        (`KismetArrayLibrary.Array_Set` (`self.EquipedItemsReference`) (`KismetMathLibrary.Conv_ByteToInt` (`local.Slot`)) _output_get true)
        (set `/Game/MyProject/MyItemSystem/Blueprints/ItemBaseClasses/NIS_BP_WorldItem.ItemInfo` (`local.l_NewItemInfo`) (`local.l_NewSpawnItem`))
        (bind _asbp_equipable_weapon (cast `/Game/MyProject/Items/EquipableItemActors/Parent/BP_Equipable_Weapon` (`local.l_NewSpawnItem`)))
        (set `/Game/MyProject/Items/EquipableItemActors/Parent/BP_Equipable_Weapon.AttachTo` self _asbp_equipable_weapon)
        (`self.CE_EquipWeapon` _asbp_equipable_weapon)))
    (elif (or (`|EnumEquality` _slot "NewEnumerator12") (`|EnumEquality` _slot "NewEnumerator13"))
      (`/Game/AdvancedLocomotionV4/Blueprints/Interfaces/ALS_Character_BPI.BPI_Set_OverlayState` "NewEnumerator0"))))

(fn `Func_OnDeath`
  (`parent.Func_OnDeath`)
  (if (`KismetSystemLibrary.IsServer`)
    (`|ExecutionSequence`
      (:`then_0`
        (for _array_element (`/Game/MyProject/MyItemSystem/Blueprints/Libraries/NIS_BFL.NIS_BFL_GetInventoriesInOrder` self)
          (for (_ _array_index) (`/Game/MyProject/MyItemSystem/Blueprints/NIS_Inventory.Pure_GetItems` _array_element)
            (`self.Server_DropItem` _array_element _array_index))))
      (:`then_1`
        (`/Game/MyProject/Blueprints/InventoryPlayerController.ROS_Respawn` (cast `/Game/MyProject/Blueprints/InventoryPlayerController` (`self.GetController`) :!pure true) 5.0)))))

(fn `FuncServer_Interact`
  (params (Hit :type "HitResult Structure"))
  (bind (_bblockinghit _binitialoverlap _time _distance _location _impactpoint _normal _impactnormal _physmat _hitactor) (`GameplayStatics.BreakHitResult` (`local.Hit`)))
  (`|ExecutionSequence`
    (:`then_0`
      (if _bblockinghit
        (if (`KismetSystemLibrary.DoesImplementInterface` _hitactor "/Game/MyProject/Blueprints/Interfaces/I_Interactable.I_Interactable_C")
          (bind _returnvalue (message `/Game/MyProject/Blueprints/Interfaces/I_Interactable.I_GetInteractDistance` _hitactor))
          (if (<= (`KismetMathLibrary.Vector_Distance` _location (`self.K2_GetActorLocation`)) _returnvalue)
            (message `/Game/MyProject/Blueprints/Interfaces/UsableActorInterface.OnActorUsed` _hitactor self)
            (return)))))
    (:`then_1`
      (`self.Server_PickupAllOverLappingItems`))))

(fn `I_GetTeamID`
  (returns (ID :type Integer))
  (return (`self.TeamID`)))

(fn `UserConstructionScript`
  (`parent.UserConstructionScript`))