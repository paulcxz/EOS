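; Consumable item effect that gradually restores health to a pawn, overriding the progress and usability functions of an effect.
; On each progress update it heals a living pawn by the difference between the maximum gain scaled by progress and the amount already given, through a heal interface message.
; The item is usable only while the pawn is valid, alive and below its final max health.
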(fn `Func_EffectProgress`
  (params (Progress :type "Float (double-precision)"))
  (locals (l_HealGainThisTime :type "Float (double-precision)" :default 0.0))
  (bind _pawn (`self.Pawn`))
  (`/Engine/EditorBlueprintResources/StandardMacros.IsValid` _pawn
    (:`Is Valid`
      (if (`/Game/MyProject/Blueprints/Pawns/Pawn_L2_AdvLocom.Pure_IsAlive` _pawn)
        (bind _output_get (set `local.l_HealGainThisTime` (- (* (`self.MaxHealthGain`) (`local.Progress`)) (`self.HealthGained`))))
        (bind _output_get_2 (set `self.HealthGained` (+ (stale _output_get_2) _output_get)))
        (message `/Game/MyProject/Blueprints/Interfaces/I_Pawn.I_Heal` (`self.Pawn`) (`local.l_HealGainThisTime`))))))

(fn `Pure_CanItemBeUsed`
  (returns (ReturnValue :type Boolean))
  (bind _pawn (`self.Pawn`))
  (`/Engine/EditorBlueprintResources/StandardMacros.IsValid` (`self.Pawn`)
    (:`Is Valid`
      (return (and (< (`.Health_17_C522567A40A5C1E5F8E4BDA48FADD811` (break `/Game/MyProject/Blueprints/Structures/S_Properties` (`/Game/MyProject/Blueprints/Pawns/Pawn_L2_AdvLocom.PawnProperties` _pawn))) (`/Game/MyProject/Blueprints/Pawns/Pawn_L2_AdvLocom.Pure_GetFinalMaxHealth` _pawn)) (`/Game/MyProject/Blueprints/Pawns/Pawn_L2_AdvLocom.Pure_IsAlive` _pawn))))
    (:`Is Not Valid`
      (return false))))

(fn `UserConstructionScript`
  (`parent.UserConstructionScript`))