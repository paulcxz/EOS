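; BP_Equipable_Weapon is an equipable weapon actor that serves as a base for held weapons.
; On equip it records the holder, disables collision on its box and mesh, and sets network ownership on the server.
; The AttachTo rep-notify stops physics and has a Pawn_L3_Actions pawn equip it right-handed, or restores physics when unattached.
; Interface getters return default ammo ID, attach type and overlay state; unequip is empty.
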(event `/Game/MyProject/Blueprints/Interfaces/I_Equipable.I_Unequiped`
  (params (Who :type "/Game/MyProject/Blueprints/Pawns/Pawn_L1_Equipment Object Reference")))

(event `/Game/MyProject/Blueprints/Interfaces/I_Equipable.I_Equiped`
  (params (Who :type "/Game/MyProject/Blueprints/Pawns/Pawn_L1_Equipment Object Reference"))
  (set `self.ItemOwner` Who)
  (`PrimitiveComponent.SetCollisionEnabled` (`self.Box`) "NoCollision")
  (`PrimitiveComponent.SetCollisionEnabled` (`self.StaticMeshComponent`) "NoCollision")
  (if (`KismetSystemLibrary.IsServer`)
    (`self.SetOwner` (`self.ItemOwner`))))

(fn `I_GetAmmoID`
  (returns (ID :type Name))
  (return "None"))

(fn `I_GetAttachType`
  (returns (AttachType :type "/Game/MyProject/Blueprints/Structures/E_AttachType Enum"))
  (return "NewEnumerator0"))

(fn `I_GetOverlayState`
  (returns (ReturnValue :type "/Game/AdvancedLocomotionV4/Data/Enums/ALS_OverlayState Enum"))
  (return "NewEnumerator0"))

(fn `OnRep_AttachTo`
  (`/Engine/EditorBlueprintResources/StandardMacros.IsValid` (`self.AttachTo`)
    (:`Is Valid`
      (`PrimitiveComponent.SetSimulatePhysics` (`self.StaticMeshComponent`) false)
      (bind _aspawn_l3_actions (cast `/Game/MyProject/Blueprints/Pawns/Pawn_L3_Actions` (`self.AttachTo`)))
      (`/Game/MyProject/Blueprints/Pawns/Pawn_L2_AdvLocom.CE_EquipWeapon` _aspawn_l3_actions self false (0.0 0.0 0.0)))
    (:`Is Not Valid`
      (`PrimitiveComponent.SetSimulatePhysics` (`self.StaticMeshComponent`) true))))

(fn `UserConstructionScript`
  (`parent.UserConstructionScript`))