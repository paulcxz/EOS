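; Blueprint function library for the NIS item system, providing shared inventory operations and queries.
; MoveItem merges matching items up to max stack size, swaps differing ones or splits stacks in half, writing through the inventory components' server setter functions.
; DropItem spawns a world item through the NIS_BP_Assistant actor and clears the slot.
; Helpers order an actor's inventories by Index, total item amounts by ID, and map equipment types to one or two slot IDs.
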(fn `NIS_BFL_DropItem`
  (params (FromInventory :type "/Game/MyProject/MyItemSystem/Blueprints/NIS_Inventory Object Reference") (Slot :type Integer))
  (returns (Result :type Boolean))
  (bind _returnvalue (`GameplayStatics.GetActorOfClass` null "/Game/MyProject/MyItemSystem/Blueprints/NIS_BP_Assistant.NIS_BP_Assistant_C"))
  (`/Game/MyProject/MyItemSystem/Blueprints/NIS_BP_Assistant.ROS_SpawnWorldItem` _returnvalue (`|GetArrayItem` (`/Game/MyProject/MyItemSystem/Blueprints/NIS_Inventory.Items` (`local.FromInventory`)) (`local.Slot`)) null)
  (bind _result (`/Game/MyProject/MyItemSystem/Blueprints/NIS_Inventory.Func_Server_SetItem` :`self` (`local.FromInventory`) :`Slot` (`local.Slot`)))
  (return _result))

(fn `NIS_BFL_GetInventoriesInOrder`
  (params (FromWho :type "Actor Object Reference"))
  (returns (Inventories :type "Array of /Game/MyProject/MyItemSystem/Blueprints/NIS_Inventory Object Reference"))
  (locals (l_Inventories :type "Array of /Game/MyProject/MyItemSystem/Blueprints/NIS_Inventory Object Reference"))
  (for _array_element (`Actor.K2_GetComponentsByClass` FromWho "/Game/MyProject/MyItemSystem/Blueprints/NIS_Inventory.NIS_Inventory_C")
    (bind _index (`/Game/MyProject/MyItemSystem/Blueprints/NIS_Inventory.Index` _array_element))
    (if (>= _index 0)
      (`KismetArrayLibrary.Array_Set` (`local.l_Inventories`) _index _array_element true)))
  (return (`local.l_Inventories`)))

(fn `NIS_BFL_GetItemTotalAmountFromActor`
  (params (FromWho :type "Actor Object Reference") (ItemID :type Name))
  (returns (Ammo :type Integer))
  (locals (l_AmmoIHave :type Integer))
  (for _array_element (`self.NIS_BFL_GetInventoriesInOrder` FromWho)
    (bind _output_get (set `local.l_AmmoIHave` (+ (stale _output_get) (`self.NIS_BFL_GetItemTotalAmountFromInv` _array_element ItemID)))))
  (return (`local.l_AmmoIHave`)))

(fn `NIS_BFL_GetItemTotalAmountFromInv`
  (params (Inventory :type "/Game/MyProject/MyItemSystem/Blueprints/NIS_Inventory Object Reference") (ItemID :type Name))
  (returns (ReturnValue :type Integer))
  (locals (l_Ret :type Integer :default 0))
  (set `local.l_Ret` 0)
  (for _array_element (`/Game/MyProject/MyItemSystem/Blueprints/NIS_Inventory.Items` Inventory)
    (bind (_valid _itemguid _definiation _currentstate) (break `/Game/MyProject/MyItemSystem/Structs/NIS_S_Item` _array_element))
    (if _valid
      (if (== (`.ID_35_21A6C172469948671FD3CB8A1BBED0DB` (break `/Game/MyProject/MyItemSystem/Structs/NIS_S_ItemDefination` _definiation)) (`local.ItemID`))
        (bind _output_get (set `local.l_Ret` (+ (stale _output_get) (`.Amount_104_5BD0F40343BC83E7582405A59DEF24E8` (break `/Game/MyProject/MyItemSystem/Structs/NIS_S_ItemCurrentState` _currentstate))))))))
  (return (`local.l_Ret`)))

(fn `NIS_BFL_GetSplitAmount`
  (params (InAmount :type Integer))
  (returns (SplitAmount :type Integer))
  (bind _returnvalue (/ InAmount 2))
  (if (== (mod InAmount 2) 0)
    (return _returnvalue)
    (else
      (return (`KismetMathLibrary.Max` (+ _returnvalue 1) _returnvalue)))))

(fn `NIS_BFL_MapSlotTypeToSlotID`
  (params (Type :type "/Game/MyProject/MyItemSystem/Structs/NIS_E_EquipmentSlotType Enum" :default "NewEnumerator2"))
  (returns (IDs :type "Array of /Game/MyProject/Blueprints/Structures/NIS_E_EquipmentSlotID Enum"))
  (locals (l_ret :type "Array of /Game/MyProject/Blueprints/Structures/NIS_E_EquipmentSlotID Enum"))
  (bind _l_ret (`local.l_ret`))
  (`KismetArrayLibrary.Array_Clear` (`local.l_ret`))
  (`|ExecutionSequence`
    (:`then_0`
      (switch `/Game/MyProject/MyItemSystem/Structs/NIS_E_EquipmentSlotType` (`local.Type`)
        (:`NewEnumerator2`
          (`KismetArrayLibrary.Array_Add` _l_ret "NewEnumerator0"))
        (:`NewEnumerator3`
          (`KismetArrayLibrary.Array_Add` _l_ret "NewEnumerator1"))
        (:`NewEnumerator4`
          (`KismetArrayLibrary.Array_Add` _l_ret "NewEnumerator2"))
        (:`NewEnumerator7`
          (`KismetArrayLibrary.Array_Add` _l_ret "NewEnumerator3"))
        (:`NewEnumerator9`
          (`KismetArrayLibrary.Array_Add` _l_ret "NewEnumerator4"))
        (:`NewEnumerator10`
          (`KismetArrayLibrary.Array_Add` _l_ret "NewEnumerator5"))
        (:`NewEnumerator17`
          (`KismetArrayLibrary.Array_Add` _l_ret "NewEnumerator6"))
        (:`NewEnumerator5`
          (`KismetArrayLibrary.Array_Add` _l_ret "NewEnumerator7"))
        (:`NewEnumerator15`
          (`KismetArrayLibrary.Array_Add` _l_ret "NewEnumerator8")
          (`KismetArrayLibrary.Array_Add` _l_ret "NewEnumerator9"))
        (:`NewEnumerator13`
          (`KismetArrayLibrary.Array_Add` _l_ret "NewEnumerator10"))
        (:`NewEnumerator16`
          (`KismetArrayLibrary.Array_Add` _l_ret "NewEnumerator11"))
        (:`NewEnumerator0`
          (`KismetArrayLibrary.Array_Add` _l_ret "NewEnumerator12"))
        (:`NewEnumerator1`
          (`KismetArrayLibrary.Array_Add` _l_ret "NewEnumerator13"))
        (:`NewEnumerator19`
          (`KismetArrayLibrary.Array_Add` _l_ret "NewEnumerator12")
          (`KismetArrayLibrary.Array_Add` _l_ret "NewEnumerator13"))))
    (:`then_1`
      (return (`local.l_ret`)))))

(fn `NIS_BFL_MoveItem`
  (params (FromInv :type "/Game/MyProject/MyItemSystem/Blueprints/NIS_Inventory Object Reference") (ToInv :type "/Game/MyProject/MyItemSystem/Blueprints/NIS_Inventory Object Reference") (FromSlot :type Integer) (ToSlot :type Integer) (Split :type Boolean))
  (returns (Result :type Boolean))
  (locals (l_FromItemInfo :type "/Game/MyProject/MyItemSystem/Structs/NIS_S_Item Structure") (l_ToItemInfo :type "/Game/MyProject/MyItemSystem/Structs/NIS_S_Item Structure") (l_SplitAmount :type Integer :default 0) (l_SplitLeftAmount :type Integer) (l_MaxStackSize :type Integer) (l_FromAmount :type Integer) (l_ToAmount :type Integer) (l_AmountCanMove :type Integer) (l_AmountAfterMoveWithoutCap :type Integer) (l_AmountWantToMove :type Integer))
  (bind _l_amountwanttomove (`local.l_AmountWantToMove`))
  (bind ((`Amount_104_5BD0F40343BC83E7582405A59DEF24E8` _amount)) (break `/Game/MyProject/MyItemSystem/Structs/NIS_S_ItemCurrentState` (`.CurrentState_12_E59680B04DB3FFA39D4B878CDD56837B` (break `/Game/MyProject/MyItemSystem/Structs/NIS_S_Item` (`local.l_FromItemInfo`)))))
  (if (or (!= (`local.FromInv`) (`local.ToInv`)) (!= (`local.FromSlot`) (`local.ToSlot`)))
    (`|ExecutionSequence`
      (:`then_0`
        (set `local.l_FromItemInfo` (`|GetArrayItem` (`/Game/MyProject/MyItemSystem/Blueprints/NIS_Inventory.Items` (`local.FromInv`)) (`local.FromSlot`)))
        (set `local.l_ToItemInfo` (`|GetArrayItem` (`/Game/MyProject/MyItemSystem/Blueprints/NIS_Inventory.Items` (`local.ToInv`)) (`local.ToSlot`)))
        (bind _output_get (set `local.l_SplitAmount` (`self.NIS_BFL_GetSplitAmount` _amount)))
        (set `local.l_SplitLeftAmount` (- _amount _output_get))
        (set `local.l_MaxStackSize` (`.MaxStackSize_105_457804EE421C991C4D20ADA6928E4B40` (break `/Game/MyProject/MyItemSystem/Structs/NIS_S_ItemDefination` (`.Definiation_2_5F261EEE43996261C586B7A249020746` (break `/Game/MyProject/MyItemSystem/Structs/NIS_S_Item` (`local.l_FromItemInfo`))))))
        (set `local.l_FromAmount` (`.Amount_104_5BD0F40343BC83E7582405A59DEF24E8` (break `/Game/MyProject/MyItemSystem/Structs/NIS_S_ItemCurrentState` (`.CurrentState_12_E59680B04DB3FFA39D4B878CDD56837B` (break `/Game/MyProject/MyItemSystem/Structs/NIS_S_Item` (`local.l_FromItemInfo`))))))
        (set `local.l_ToAmount` (`.Amount_104_5BD0F40343BC83E7582405A59DEF24E8` (break `/Game/MyProject/MyItemSystem/Structs/NIS_S_ItemCurrentState` (`.CurrentState_12_E59680B04DB3FFA39D4B878CDD56837B` (break `/Game/MyProject/MyItemSystem/Structs/NIS_S_Item` (`local.l_ToItemInfo`))))))
        (bind _output_get_2 (set `local.l_AmountWantToMove` (select `bool` (`local.Split`) :`false` (`local.l_FromAmount`) :`true` (`local.l_SplitAmount`))))
        (bind _output_get_3 (set `local.l_AmountAfterMoveWithoutCap` (+ _output_get_2 (`local.l_ToAmount`))))
        (set `local.l_AmountCanMove` (select `bool` (> _output_get_3 (`local.l_MaxStackSize`)) :`false` _l_amountwanttomove :`true` (- _l_amountwanttomove (- (`local.l_AmountAfterMoveWithoutCap`) (`local.l_MaxStackSize`))))))
      (:`then_1`
        (if (`.Valid_10_A5F4438E4CED4CA4C4B5889683E540DA` (break `/Game/MyProject/MyItemSystem/Structs/NIS_S_Item` (`local.l_FromItemInfo`)))
          (if (`.Valid_10_A5F4438E4CED4CA4C4B5889683E540DA` (break `/Game/MyProject/MyItemSystem/Structs/NIS_S_Item` (`local.l_ToItemInfo`)))
            (if (== (`.ID_35_21A6C172469948671FD3CB8A1BBED0DB` (break `/Game/MyProject/MyItemSystem/Structs/NIS_S_ItemDefination` (`.Definiation_2_5F261EEE43996261C586B7A249020746` (break `/Game/MyProject/MyItemSystem/Structs/NIS_S_Item` (`local.l_ToItemInfo`))))) (`.ID_35_21A6C172469948671FD3CB8A1BBED0DB` (break `/Game/MyProject/MyItemSystem/Structs/NIS_S_ItemDefination` (`.Definiation_2_5F261EEE43996261C586B7A249020746` (break `/Game/MyProject/MyItemSystem/Structs/NIS_S_Item` (`local.l_FromItemInfo`))))))
              (`/Game/MyProject/MyItemSystem/Blueprints/NIS_Inventory.Func_Server_SetItemAmount` (`local.ToInv`) (`local.ToSlot`) (+ (`local.l_AmountCanMove`) (`local.l_ToAmount`)))
              (`/Game/MyProject/MyItemSystem/Blueprints/NIS_Inventory.Func_Server_SetItemAmount` (`local.FromInv`) (`local.FromSlot`) (- (`local.l_FromAmount`) (`local.l_AmountCanMove`)))
              (elif (not (`local.Split`))
                (`/Game/MyProject/MyItemSystem/Blueprints/NIS_Inventory.Func_Server_SetItem` (`local.ToInv`) (`local.ToSlot`) (`local.l_FromItemInfo`)) ; No spliting not the same items, swap them
                (`/Game/MyProject/MyItemSystem/Blueprints/NIS_Inventory.Func_Server_SetItem` (`local.FromInv`) (`local.FromSlot`) (`local.l_ToItemInfo`)) ; No spliting not the same items, swap them
              ))
            (else
              (bind _result (`/Game/MyProject/MyItemSystem/Blueprints/NIS_Inventory.Func_Server_SetItem` (`local.ToInv`) (`local.ToSlot`) (`local.l_FromItemInfo`))) ; Set item to target slot
              (if _result
                (if (`local.Split`)
                  (`/Game/MyProject/MyItemSystem/Blueprints/NIS_Inventory.Func_Server_SetItemAmount` (`local.ToInv`) (`local.ToSlot`) (`local.l_SplitAmount`))
                  (`/Game/MyProject/MyItemSystem/Blueprints/NIS_Inventory.Func_Server_SetItemAmount` (`local.FromInv`) (`local.FromSlot`) (`local.l_SplitLeftAmount`))
                  (else
                    (`/Game/MyProject/MyItemSystem/Blueprints/NIS_Inventory.Func_Server_SetItem` :`self` (`local.FromInv`) :`Slot` (`local.FromSlot`))))
                (else
                  (return true)))))
          (else
            (return false)))))
    (else
      (return false))))