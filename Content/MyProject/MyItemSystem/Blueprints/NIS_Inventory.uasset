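; NIS_Inventory is an item container component that serves as either a general inventory or an equipment inventory, using a slot array sized at BeginPlay.
; Adding an item without a specified slot fills the first free slot, or in equipment mode a free slot matching its equipment type, then messages the owner through an interface.
; Server-named functions also overwrite slots or change amounts, clearing a slot when the amount drops to zero or below.
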(event `self.ReceiveBeginPlay`
  (for _ (range (`self.InventorySize`))
    (`KismetArrayLibrary.Array_Add` (`self.Items`))))

(fn `Func_Server_AddItem`
  (params (NewItem :type "/Game/MyProject/MyItemSystem/Structs/NIS_S_Item Structure (by ref)") (Slot :type Integer :default -1))
  (returns (Result :type Boolean))
  (bind (_newitem_valid _newitem_itemguid _newitem_definiation _newitem_currentstate) (break `/Game/MyProject/MyItemSystem/Structs/NIS_S_Item` (`local.NewItem`)))
  (bind (_newitem_valid_2 _newitem_itemguid_2 _newitem_definiation_2 _newitem_currentstate_2) (break `/Game/MyProject/MyItemSystem/Structs/NIS_S_Item` (`local.NewItem`)))
  (bind ((`ItemType_136_6F65BDF74AF3950358D25783E49E9C6F` _itemtype) (`EquipmentSlot_137_2DD3EC7D4ADC51E425F2C4BEB9CB572A` _equipmentslot)) (break `/Game/MyProject/MyItemSystem/Structs/NIS_S_ItemDefination` (`.Definiation_2_5F261EEE43996261C586B7A249020746` (break `/Game/MyProject/MyItemSystem/Structs/NIS_S_Item` (`local.NewItem`)))))
  (if (< (`local.Slot`) 0)
    (if (`self.IsEquipmentInv`)
      (if (`|EnumEquality` _itemtype "NewEnumerator1")
        (for _array_element (`/Game/MyProject/MyItemSystem/Blueprints/Libraries/NIS_BFL.NIS_BFL_MapSlotTypeToSlotID` _equipmentslot)
          (bind _returnvalue (`KismetMathLibrary.Conv_ByteToInt` _array_element))
          (if (not (`.Valid_10_A5F4438E4CED4CA4C4B5889683E540DA` (break `/Game/MyProject/MyItemSystem/Structs/NIS_S_Item` (`|GetArrayItem` (`self.Items`) _returnvalue))))
            (`KismetArrayLibrary.Array_Set` (`self.Items`) _returnvalue (make `/Game/MyProject/MyItemSystem/Structs/NIS_S_Item` true _newitem_itemguid _newitem_definiation _newitem_currentstate))
            (message `/Game/MyProject/Blueprints/Interfaces/I_EquippedPawn.I_EquipmentChanged` (`self.GetOwner`) _array_element)
            (return true)))
        (return false)
        (else
          (return false)))
      (else
        (for (_array_element_2 _array_index) (`self.Items`)
          (if (not (`.Valid_10_A5F4438E4CED4CA4C4B5889683E540DA` (break `/Game/MyProject/MyItemSystem/Structs/NIS_S_Item` _array_element_2)))
            (`KismetArrayLibrary.Array_Set` (`self.Items`) _array_index (make `/Game/MyProject/MyItemSystem/Structs/NIS_S_Item` true _newitem_itemguid_2 _newitem_definiation_2 _newitem_currentstate_2))
            (return true)))
        (return false)))
    (else
      (return false))))

(fn `Func_Server_SetItem`
  (params (Slot :type Integer) (ItemInfo :type "/Game/MyProject/MyItemSystem/Structs/NIS_S_Item Structure"))
  (returns (Result :type Boolean))
  (if (`KismetArrayLibrary.Array_IsValidIndex` (`self.Items`) Slot)
    (`KismetArrayLibrary.Array_Set` (`self.Items`) (`local.Slot`) (`local.ItemInfo`))
    (return true)
    (else
      (return false))))

(fn `Func_Server_SetItemAmount`
  (params (Slot :type Integer) (NewAmount :type Integer))
  (returns (Result :type Boolean))
  (bind _output (`|GetArrayItem` (`self.Items`) (`local.Slot`)))
  (bind (_valid _itemguid _definiation _currentstate) (break `/Game/MyProject/MyItemSystem/Structs/NIS_S_Item` _output))
  (if (`KismetArrayLibrary.Array_IsValidIndex` (`self.Items`) Slot)
    (if (> (`local.NewAmount`) 0)
      (if (`.Valid_10_A5F4438E4CED4CA4C4B5889683E540DA` (break `/Game/MyProject/MyItemSystem/Structs/NIS_S_Item` _output))
        (setmembers `/Game/MyProject/MyItemSystem/Structs/NIS_S_Item` :`StructRef` _output :`CurrentState` (make `/Game/MyProject/MyItemSystem/Structs/NIS_S_ItemCurrentState` (break `/Game/MyProject/MyItemSystem/Structs/NIS_S_ItemCurrentState` _currentstate) (`local.NewAmount`) (`.RandomizedPropBounce_144_C7847BCA4F2E2B52E29F93ADCC5D1D6D` (break `/Game/MyProject/MyItemSystem/Structs/NIS_S_ItemCurrentState` _currentstate))))
        (return true))
      (else
        (`self.Func_Server_SetItem` (`local.Slot`))))
    (else
      (return false))))